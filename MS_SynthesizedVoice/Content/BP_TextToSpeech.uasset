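; BP_TextToSpeech is a prototype speech synthesizer; on BeginPlay it decodes a hardcoded TIPA phonetic string and prints the tokens and IPA.
; TIPADecoder keeps brace macros as single tokens and maps them to IPA, passing unknown tokens through.
; An unconnected test sequence feeds formants to MSTextToSpeech, voicing allophones found in the formant map and using breath noise otherwise.
; Input actions only set Allophone; their mapping context setup is also unconnected.
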(event Input|EnhancedActionEvents|EnhancedInputActionIA_ae
  (params (ActionValue :type Boolean) (ElapsedSeconds :type Float%20%28double-precision%29) (TriggeredSeconds :type Float%20%28double-precision%29) (InputAction :type Input%20Action%20Object%20Reference :default "/Game/Controls/IA_ae.IA_ae"))
  (:Triggered
    (Variables|Default|SetAllophone "/ae")))

(event Input|EnhancedActionEvents|EnhancedInputActionIA_i
  (params (ActionValue :type Boolean) (ElapsedSeconds :type Float%20%28double-precision%29) (TriggeredSeconds :type Float%20%28double-precision%29) (InputAction :type Input%20Action%20Object%20Reference :default "/Game/Controls/IA_i.IA_i"))
  (:Triggered
    (Variables|Default|SetAllophone "i")))

(event Input|EnhancedActionEvents|EnhancedInputActionIA_u
  (params (ActionValue :type Boolean) (ElapsedSeconds :type Float%20%28double-precision%29) (TriggeredSeconds :type Float%20%28double-precision%29) (InputAction :type Input%20Action%20Object%20Reference :default "/Game/Controls/IA_u.IA_u"))
  (:Triggered
    (Variables|Default|SetAllophone "u")))

(event EventBeginPlay
  (CallFunction|TIPADecoder (Utilities|String|MakeLiteralString "bA{textbeltl}"))
  (for _array_element (Variables|Default|GetDecodedTIPA)
    (Development|PrintString _array_element))
  (Development|PrintString (Variables|Default|GetIPA)))

(fn ConstructionScript)

(fn TIPADecoder
  (params (TIPA :type String))
  (Utilities|Array|Clear (Variables|Default|GetDecodedTIPA))
  (Variables|Default|SetIPA "")
  (for _array_element (Utilities|String|GetCharacterArrayfromString TIPA)
    (Variables|Default|SetCurrentTIPA (Utilities|String|Append (Variables|Default|GetCurrentTIPA) _array_element))
    (if (Class|KismetMathLibrary|XORBoolean (or (Utilities|Enum|Equal(Enum) _array_element "{") (Variables|Default|GetMacro)) (Utilities|Enum|Equal(Enum) _array_element "}"))
      (Variables|Default|SetMacro true)
      (else
        (Variables|Default|SetMacro false)
        (Utilities|Array|Add (Variables|Default|GetDecodedTIPA) (Variables|Default|GetCurrentTIPA))
        (Variables|Default|SetIPA (Utilities|String|Append (Variables|Default|GetIPA) (Utilities|String|SelectString (.Value (Utilities|Map|Find (Variables|Default|GetTIPAToIPA) (Variables|Default|GetCurrentTIPA))) (Variables|Default|GetCurrentTIPA) (.ReturnValue (Utilities|Map|Find (Variables|Default|GetTIPAToIPA) (Variables|Default|GetCurrentTIPA))))))
        (Variables|Default|SetCurrentTIPA ""))))
  (return))