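; Text-to-speech prototype Blueprint that feeds formant data for a hard-coded phrase to a MetaSound-style audio component on BeginPlay.
; The phrase is either direct IPA or X-SAMPA, transcribed through DT_Allophones columns with backslash-suffixed symbols handled.
; Each IPA character looks up its row's three formants, which fill float arrays sent as audio parameters before a cue trigger.
; A TIPA decoder exists but is uncalled, with its parsing loop disconnected.
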(event EventBeginPlay
  (bind _returnvalue (Utilities|String|MakeLiteralString "{iu"))
  (switch Utilities|FlowControl|Switch|SwitchonE_Transcriber "NewEnumerator1"
    (:NewEnumerator0
      (Variables|Default|SetPhrase_IPA _returnvalue))
    (:NewEnumerator1
      (CallFunction|X-SAMPATranscriber _returnvalue)))
  (Audio|Components|Audio|Play (Variables|Default|GetMS_TextToSpeech) 0.0)
  (for _array_element (Utilities|String|GetCharacterArrayfromString (Variables|Default|GetPhrase_IPA))
    (Development|PrintString _array_element)
    (bind _returnvalue_2 (Utilities|GetDataTableRow "/Game/DT_Allophones.DT_Allophones" (Utilities|String|StringToName _array_element))
      (:then
        (Utilities|Array|Add (Variables|Default|GetPhrase_F1) (.x (.Formants (Utilities|Struct|BreakF_Allophones _returnvalue_2))))
        (Utilities|Array|Add (Variables|Default|GetPhrase_F2) (.y (.Formants (Utilities|Struct|BreakF_Allophones _returnvalue_2))))
        (Utilities|Array|Add (Variables|Default|GetPhrase_F3) (.z (.Formants (Utilities|Struct|BreakF_Allophones _returnvalue_2)))))))
  (Class|AudioParameterControllerInterface|SetFloatArrayParameter (Variables|Default|GetMS_TextToSpeech) "Phrase_F1" (Variables|Default|GetPhrase_F1))
  (Class|AudioParameterControllerInterface|SetFloatArrayParameter (Variables|Default|GetMS_TextToSpeech) "Phrase_F2" (Variables|Default|GetPhrase_F2))
  (Class|AudioParameterControllerInterface|SetFloatArrayParameter (Variables|Default|GetMS_TextToSpeech) "Phrase_F3" (Variables|Default|GetPhrase_F3))
  (Class|AudioParameterControllerInterface|SetTriggerParameter (Variables|Default|GetMS_TextToSpeech) "CueArrays"))

(fn ConstructionScript)

(fn TIPADecoder
  (params (TIPA :type String))
  (Utilities|Array|Clear (Variables|Default|GetDecodedTIPA))
  (Variables|Default|SetPhrase_IPA "")
  (Class|DataTableFunctionLibrary|GetDataTableColumnasString "/Game/DT_Allophones.DT_Allophones" "TIPA"))

(fn X-SAMPATranscriber
  (params (Phrase_X-SAMPA :type String))
  (Variables|Default|SetPhrase_IPA "")
  (for _array_element (Utilities|String|GetCharacterArrayfromString Phrase_X-SAMPA)
    (if (Utilities|Enum|Equal(Enum) _array_element "\\")
      (Variables|Default|SetAllophone%20Collection (Utilities|String|Append (Variables|Default|GetAllophone%20Collection) _array_element))
      (bind _returnvalue (Class|DataTableFunctionLibrary|GetDataTableColumnasString "/Game/DT_Allophones.DT_Allophones" "X-SAMPA" :!label _label))
      (bind _returnvalue_2 (Class|DataTableFunctionLibrary|GetDataTableColumnasString "/Game/DT_Allophones.DT_Allophones" "IPA"))
      (Variables|Default|SetPhrase_IPA (Utilities|String|Append (Variables|Default|GetPhrase_IPA) (Utilities|String|SelectString (Utilities|Array|Get(acopy) _returnvalue_2 (Utilities|Array|FindItem _returnvalue (Variables|Default|GetAllophone%20Collection))) (Variables|Default|GetAllophone%20Collection) (Utilities|Enum|Equal(Enum) (Utilities|Array|Get(acopy) _returnvalue (Utilities|Array|FindItem _returnvalue (Variables|Default|GetAllophone%20Collection))) (Variables|Default|GetAllophone%20Collection)))))
      (Variables|Default|SetAllophone%20Collection "")
      (else
        (Utilities|FlowControl|Sequence
          (:then_0
            (if (not (Utilities|Enum|Equal(Enum) (Variables|Default|GetAllophone%20Collection) ""))
              (goto _label)))
          (:then_1
            (Variables|Default|SetAllophone%20Collection _array_element))))))
  (bind _returnvalue_3 (Class|DataTableFunctionLibrary|GetDataTableColumnasString "/Game/DT_Allophones.DT_Allophones" "X-SAMPA"))
  (bind _returnvalue_4 (Class|DataTableFunctionLibrary|GetDataTableColumnasString "/Game/DT_Allophones.DT_Allophones" "IPA"))
  (Variables|Default|SetPhrase_IPA (Utilities|String|Append (Variables|Default|GetPhrase_IPA) (Utilities|String|SelectString (Utilities|Array|Get(acopy) _returnvalue_4 (Utilities|Array|FindItem _returnvalue_3 (Variables|Default|GetAllophone%20Collection))) (Variables|Default|GetAllophone%20Collection) (Utilities|Enum|Equal(Enum) (Utilities|Array|Get(acopy) _returnvalue_3 (Utilities|Array|FindItem _returnvalue_3 (Variables|Default|GetAllophone%20Collection))) (Variables|Default|GetAllophone%20Collection)))))
  (Variables|Default|SetAllophone%20Collection ""))